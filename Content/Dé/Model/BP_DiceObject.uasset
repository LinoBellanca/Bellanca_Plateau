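; BP_DiceObject is a die actor that works out which face landed up, then destroys itself.
; After BeginPlay it samples its location at intervals, repeating until the position stops changing.
; It then loops over six face components to find the one whose forward vector points world up within a tolerance.
; That index plus one becomes DiceResult, CanShowRes is set, and the actor is destroyed after a short delay.
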(event `self.ReceiveBeginPlay`
  (`KismetSystemLibrary.Delay` 2.0)
  (`self.HasStopped`))

(event `HasStopped`
  (set `self.DiceLocation` (`self.K2_GetActorLocation`))
  (`KismetSystemLibrary.Delay` 4.0)
  (if (== (`self.DiceLocation`) (`self.K2_GetActorLocation`) :`ErrorTolerance` 0.001)
    (`self.Result`)
    (else
      (`self.HasStopped`))))

(event `Result`
  (for (_array_element _array_index) (`|MakeArray` (`self.Face1`) (`self.Face2`) (`self.Face3`) (`self.Face4`) (`self.Face5`) (`self.Face6`))
    (if (== (`SceneComponent.GetForwardVector` _array_element) (0.0 0.0 1.0) :`ErrorTolerance` 0.05)
      (break)))
  (set `self.DiceResult` (+ _array_index 1))
  (set `self.CanShowRes` true)
  (if true
    (`KismetSystemLibrary.Delay` 0.2)
    (`self.K2_DestroyActor`)))

(fn `UserConstructionScript`)