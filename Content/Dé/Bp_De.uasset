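; Dice actor Blueprint that rolls a configurable number of dice with a configurable number of sides.
; RollDice starts ActualDiceResult at DiceNumber, then adds a random value from 1 to DiceType for each die, so the total includes the die count on top of the rolls.
; The event graph and construction script are empty, and a debug print of the result is disconnected.
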(event `self.ReceiveBeginPlay`)

(event `self.ReceiveTick`
  (params (DeltaSeconds :type "Float (single-precision)")))

(fn `RollDice`
  (set `self.ActualDiceResult` (`self.DiceNumber`))
  (for _ (range 1 (+ (`self.DiceNumber`) 1))
    (bind _output_get (set `self.ActualDiceResult` (+ (`self.ActualDiceResult`) (`KismetMathLibrary.RandomIntegerInRange` 1 (`self.DiceType`)))))))

(fn `UserConstructionScript`)