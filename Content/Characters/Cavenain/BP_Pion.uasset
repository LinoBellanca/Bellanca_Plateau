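; BP_Pion is a player's game piece that walks between board cells using AI Move To, aiming slightly above each cell.
; It caches the game instance and game mode on BeginPlay.
; MoveToNewCell moves directly to a cell.
; MoveToTempCell starts a move to an intermediate cell, then after a short delay, without waiting for arrival, calls the game mode's MovePion with the final cell and current player ID.
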(event `self.ReceiveBeginPlay`
  (bind _asbp_game_instance (cast `/Game/Game/BP_GameInstance` (`GameplayStatics.GetGameInstance`)))
  (set `self.As BP Game Instance` _asbp_game_instance)
  (bind _asbp_game_mode (cast `/Game/Game/BP_GameMode` (`GameplayStatics.GetGameMode`)))
  (set `self.As BP Game Mode` _asbp_game_mode))

(event `MoveToNewCell`
  (params (NewCellPosition :type "Vector Structure"))
  (`|AIMoveTo` self (+ NewCellPosition (0.0 0.0 100.0)) null))

(event `MoveToTempCell`
  (params (CellLocation :type "Vector Structure") (FinalCell :type Integer))
  (bind _as_bp_game_mode (`self.As BP Game Mode`))
  (`|AIMoveTo` self (+ CellLocation (0.0 0.0 100.0)) null
    (:`then`
      (`KismetSystemLibrary.Delay` 0.5)
      (`/Game/Game/BP_GameMode.MovePion` _as_bp_game_mode FinalCell (`/Game/Game/BP_GameMode.PlayerIDToPlay` _as_bp_game_mode)))))

(fn `UserConstructionScript`)