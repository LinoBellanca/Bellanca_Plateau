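; Game mode for a dice board game that spawns pawns and runs player turns.
; On BeginPlay it spawns one pawn per GameInstance player, scattered around player 0's cell, plus the die.
; CyclePlayers calls RollADiceAndMove, which updates the stored cell and moves the pawn, showing the end-game widget at cell 15.
; Turns advance by incrementing or wrapping the current pawn's PionID, then indexing GetAllActorsOfClass with it.
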(event `self.ReceiveBeginPlay`
  (bind _asbp_game_instance (cast `/Game/Pion/BP_GameInstance` (`GameplayStatics.GetGameInstance`)))
  (bind _output_get (set `self.As BP Game Instance` _asbp_game_instance))
  (bind _playercellnumber (`/Game/Pion/BP_GameInstance.GetPlayerCellNumberByPlayerID` _output_get 0))
  (`KismetSystemLibrary.Delay` 0.5)
  (bind _celllocation (`/Game/CaseEtPlateau/BP_Board.GetCellPositionByNumber` (`self.Plateau`) _playercellnumber))
  (for (_ _array_index) (`/Game/Pion/BP_GameInstance.PlayerList` (`self.As BP Game Instance`))
    (bind _returnvalue (`|SpawnActorFromClass` "/Game/Pion/BP_Pion.BP_Pion_C" (`KismetMathLibrary.MakeTransform` (`KismetMathLibrary.MakeVector` (+ (`KismetMathLibrary.RandomFloatInRange` -50.0 50.0) (.x _celllocation)) (+ (`KismetMathLibrary.RandomFloatInRange` -50.0 50.0) (.y _celllocation)) (.z _celllocation))) "Undefined" "MultiplyWithRoot" null null))
    (bind _output_get_2 (set `self.PionPlayer` _returnvalue))
    (set `/Game/Pion/BP_Pion.PionID` _array_index _output_get_2)
    (`KismetSystemLibrary.Delay` 0.2))
  (bind _returnvalue_2 (`|SpawnActorFromClass` "/Game/Dé/Bp_De.Bp_De_C" (`KismetMathLibrary.MakeTransform` (0.0 0.0 0.0)) "Undefined" "MultiplyWithRoot" null null))
  (set `self.Dice` _returnvalue_2)
  (bind _outactors (`GameplayStatics.GetAllActorsOfClass` "/Game/Pion/BP_Pion.BP_Pion_C"))
  (set `self.PionPlayer` (`|GetArrayItem` _outactors)))

(event `GetCellList`
  (params (IndexCase :type Integer))
  ;[1 1 1] Ancienne méthode de spawn
  (`|SpawnActorFromClass` "/Game/Pion/BP_Pion.BP_Pion_C" (`KismetMathLibrary.MakeTransform` (`self.K2_GetActorLocation` (`|GetArrayItem` (`/Game/CaseEtPlateau/BP_Board.CellList` (`self.Plateau`)) IndexCase))) "Undefined" "MultiplyWithRoot" null null))

(fn `CyclePlayers`
  (bind _pionplayer (`self.PionPlayer`))
  (bind _pionid (`/Game/Pion/BP_Pion.PionID` _pionplayer))
  (`KismetSystemLibrary.PrintString` (`KismetStringLibrary.Conv_IntToString` _pionid))
  (`self.RollADiceAndMove` (`|GetArrayItem` (`/Game/Pion/BP_GameInstance.PlayerList` (`self.As BP Game Instance`)) _pionid))
  (if (>= (`/Game/Pion/BP_Pion.PionID` _pionplayer) (- (`KismetArrayLibrary.Array_Length` (`/Game/Pion/BP_GameInstance.PlayerList` (`self.As BP Game Instance`))) 1))
    (bind _output_get (set `/Game/Pion/BP_Pion.PionID` 0 _pionplayer))
    (bind _outactors (`GameplayStatics.GetAllActorsOfClass` "/Game/Pion/BP_Pion.BP_Pion_C"))
    (set `self.PionPlayer` (`|GetArrayItem` _outactors _output_get))
    (else
      (bind _output_get_2 (set `/Game/Pion/BP_Pion.PionID` (+ (`/Game/Pion/BP_Pion.PionID` _pionplayer) 1) _pionplayer))
      (bind _outactors_2 (`GameplayStatics.GetAllActorsOfClass` "/Game/Pion/BP_Pion.BP_Pion_C"))
      (set `self.PionPlayer` (`|GetArrayItem` _outactors_2 _output_get_2)))))

(fn `RollADiceAndMove`
  (params (ArrayResult :type "/Game/Pion/S_PlayerData Structure"))
  (bind _playerid (break `/Game/Pion/S_PlayerData` ArrayResult))
  (bind _dice (`self.Dice`))
  (bind _as_bp_game_instance (`self.As BP Game Instance`))
  (`/Game/Dé/Bp_De.RollDice` _dice)
  (bind _playercellnumber (`/Game/Pion/BP_GameInstance.GetPlayerCellNumberByPlayerID` _as_bp_game_instance _playerid))
  (bind _returnvalue (+ _playercellnumber (`/Game/Dé/Bp_De.ActualDiceResult` _dice)))
  (`/Game/Pion/BP_GameInstance.SetPlayerCellNumberByPlayerID` _as_bp_game_instance _playerid _returnvalue)
  (if (>= _returnvalue 15)
    ;[1 1 1] Quand j'arrive à la dernière case
    (bind _output_get (set `/Game/Dé/Bp_De.ActualDiceResult` 15 (`self.Dice`)))
    (`/Game/Pion/BP_GameInstance.SetPlayerCellNumberByPlayerID` (`self.As BP Game Instance`) _playerid _output_get)
    (bind _celllocation (`/Game/CaseEtPlateau/BP_Board.GetCellPositionByNumber` (`self.Plateau`) _output_get))
    (`/Game/Pion/BP_Pion.MoveToNewCell` (`self.PionPlayer`) _celllocation _output_get)
    (bind _returnvalue_2 (`|CreateWidget` "/Game/Widgets/WB_EndGame.WB_EndGame_C"))
    (`UserWidget.AddToViewport` _returnvalue_2 0)
    (set `PlayerController.bShowMouseCursor` true (`GameplayStatics.GetPlayerController` 0))
    (else
      (bind _celllocation_2 (`/Game/CaseEtPlateau/BP_Board.GetCellPositionByNumber` (`self.Plateau`) _returnvalue))
      (`/Game/Pion/BP_Pion.MoveToNewCell` (`self.PionPlayer`) _celllocation_2 _output_get))))

(fn `UserConstructionScript`)