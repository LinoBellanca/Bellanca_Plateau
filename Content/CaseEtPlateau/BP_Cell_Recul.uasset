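; BP_Cell_Recul is a board cell that sends the player's pawn backward ("Recul").
; Its Action override calls the parent, reads the player's cell number from the game instance and stores it as the game mode's ActualCellNumber.
; It then prints "Recul" and calls the game mode's MovePion to the current cell minus NbrCaseEnMoins.
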(fn `Action`
  (params (PlayerID :type Integer))
  (`parent.Action` PlayerID)
  (bind _playercellnumber (`/Game/Game/BP_GameInstance.GetPlayerCellNumberByPlayerID` (`self.As BP Game Instance`) PlayerID))
  (set `/Game/Game/BP_GameMode.ActualCellNumber` _playercellnumber (`self.As BP Game Mode`))
  (`KismetSystemLibrary.PrintString` "Recul")
  (`/Game/Game/BP_GameMode.MovePion` (`self.As BP Game Mode`) (- _playercellnumber (`self.NbrCaseEnMoins`)) PlayerID))

(fn `UserConstructionScript`
  (`parent.UserConstructionScript`))