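; BP_DodoSpawn is a spawner actor that endlessly spawns dodoes at its own transform, starting on BeginPlay.
; A self-recalling event waits a random delay between the min and max settings, then spawns either BP_DodoKing, by a percentage-style chance roll, or a regular BP_Dodo.
; A parallel timed loop periodically decrements the maximum delay with no lower clamp, so spawning speeds up over time.
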(event `self.ReceiveBeginPlay`
  (`self.SpawnDodoes`)
  (`self.HurrySpawn`))

(event `SpawnDodoes`
  (`KismetSystemLibrary.Delay` (`KismetMathLibrary.RandomFloatInRange` (`self.MinDelayForSpawn`) (`self.MaxDelayForSpawn`)))
  (if (< (`KismetMathLibrary.RandomIntegerInRange` 0 100) (`self.ChanceForKingToSpawn`))
    (`|SpawnActorFromClass` "/Game/Collect/Collectible/BP_DodoKing.BP_DodoKing_C" (`self.GetTransform`) "Undefined" "MultiplyWithRoot" null null)
    (else
      (`|SpawnActorFromClass` "/Game/Collect/Collectible/BP_Dodo.BP_Dodo_C" (`self.GetTransform`) "Undefined" "MultiplyWithRoot" null null)))
  (`self.SpawnDodoes`))

(event `HurrySpawn`
  (`KismetSystemLibrary.Delay` 5.0)
  (`/Engine/EditorBlueprintResources/StandardMacros.DecrementFloat` (`self.MaxDelayForSpawn`)
    (:`  `
      (`self.HurrySpawn`))))

(fn `UserConstructionScript`)