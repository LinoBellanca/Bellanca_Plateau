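; BP_DodoKing is a collectible AI character in the Collect game that flees from players and awards points when caught.
; It roams to random reachable points until a collect character enters its Sphere, then speeds up and repeatedly moves directly away from that player.
; Leaving the Sphere restores normal speed and roaming.
; DeathZone overlap with either player adds its value to that player's score through the game mode and destroys it.
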(event `self.ReceiveBeginPlay`
  (bind _asbp_collect_gm (cast `/Game/Collect/Blueprints/BP_CollectGM` (`GameplayStatics.GetGameMode`)))
  (set `self.As BP Collect GM` _asbp_collect_gm)
  (`self.Random Roam`))

(event `Run Away`
  (bind _returnvalue (`self.K2_GetActorLocation`))
  (`|AIMoveTo` self (`KismetMathLibrary.MakeVector` (.x (+ _returnvalue (* (`KismetMathLibrary.GetForwardVector` (`KismetMathLibrary.FindLookAtRotation` _returnvalue (`self.K2_GetActorLocation` (`self.PlayerToRunFrom`)))) -500.0))) (.y (+ _returnvalue (* (`KismetMathLibrary.GetForwardVector` (`KismetMathLibrary.FindLookAtRotation` _returnvalue (`self.K2_GetActorLocation` (`self.PlayerToRunFrom`)))) -500.0))) (.z _returnvalue)) null
    (:`OnSuccess`
      _)
    (:`OnFail`
      _))
  (`self.Run Away`))

(event `self.Sphere.OnComponentBeginOverlap`
  (params (OverlappedComponent :type "PrimitiveComponent Object Reference") (OtherActor :type "Actor Object Reference") (OtherComp :type "PrimitiveComponent Object Reference") (OtherBodyIndex :type Integer) (bFromSweep :type Boolean) (SweepResult :type "HitResult Structure (by ref)"))
  (bind _asbp_collect_character (cast `/Game/Collect/Blueprints/BP_CollectCharacter` OtherActor))
  (set `self.PlayerToRunFrom` _asbp_collect_character)
  (set `CharacterMovementComponent.MaxWalkSpeed` 2000.0 (`self.CharacterMovement`))
  (`self.Run Away`))

(event `self.Sphere.OnComponentEndOverlap`
  (params (OverlappedComponent :type "PrimitiveComponent Object Reference") (OtherActor :type "Actor Object Reference") (OtherComp :type "PrimitiveComponent Object Reference") (OtherBodyIndex :type Integer))
  (set `CharacterMovementComponent.MaxWalkSpeed` 600.0 (`self.CharacterMovement`))
  (`self.Random Roam`))

(event `Random Roam`
  (`|AIMoveTo` self (`NavigationSystemV1.K2_GetRandomReachablePointInRadius` (`self.K2_GetActorLocation`) 2500.0 null null) null
    (:`OnSuccess`
      (`self.Random Roam`))))

(event `self.DeathZone.OnComponentBeginOverlap`
  (params (OverlappedComponent :type "PrimitiveComponent Object Reference") (OtherActor :type "Actor Object Reference") (OtherComp :type "PrimitiveComponent Object Reference") (OtherBodyIndex :type Integer) (bFromSweep :type Boolean) (SweepResult :type "HitResult Structure (by ref)"))
  (cast `/Game/Collect/Blueprints/BP_P1` OtherActor
    (:`then`
      (`/Game/Collect/Blueprints/BP_CollectGM.AddScore1` (`self.As BP Collect GM`) (`self.ValueToGive`))
      (`self.K2_DestroyActor`))
    (:`CastFailed`
      (cast `/Game/Collect/Blueprints/BP_P2` OtherActor)
      (`/Game/Collect/Blueprints/BP_CollectGM.AddScore2` (`self.As BP Collect GM`) (`self.ValueToGive`))
      (`self.K2_DestroyActor`))))

(fn `UserConstructionScript`)