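; BP_Carte is a memory game card, a stone slab whose cube material is set from its animal CardType in the construction script.
; A click on a clickable slab toggles clickability and flips it, then notifies BP_MemoManager after a delay.
; ToggleCard checks the slab's world pitch to choose turn or reset, each a timeline that offsets location, drives pitch and updates IsTurned.
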(event `self.ReceiveBeginPlay`
  (bind _returnvalue (`GameplayStatics.GetActorOfClass` "/Game/Memory/BP_MemoManager.BP_MemoManager_C"))
  (set `self.MemoManager` _returnvalue))

(event `Turn Card`
  (bind (_returnvalue_location _returnvalue_rotation) (`KismetMathLibrary.BreakTransform` (`SceneComponent.GetRelativeTransform` (`self.stone_slab`))))
  (set `self.CardLocation` _returnvalue_location)
  (set `self.CardRotation` _returnvalue_rotation)
  (bind (_direction _location _rotation) (`Timeline|CardTurning` :!via `PlayFromStart`)
    (:`Update`
      (`SceneComponent.K2_SetRelativeLocation` (`self.stone_slab`) (+ _location (`self.CardLocation`)) false false)
      (`SceneComponent.K2_SetRelativeRotation` (`self.stone_slab`) (`KismetMathLibrary.MakeRotator` 0.0 _rotation) false false)
      (set `self.IsTurned` true))))

(event `self.stone_slab.OnClicked`
  (params (TouchedComponent :type "PrimitiveComponent Object Reference") (ButtonPressed :type "Key Structure"))
  (if (`self.IsClickable`)
    (`self.ToggleCard`)
    (`KismetSystemLibrary.Delay` 3.0)
    (`/Game/Memory/BP_MemoManager.OnCardClicked` (`self.MemoManager`) self)))

(event `Reset Card`
  (bind (_returnvalue_location _returnvalue_rotation) (`KismetMathLibrary.BreakTransform` (`SceneComponent.GetRelativeTransform` (`self.stone_slab`))))
  (set `self.CardLocation` _returnvalue_location)
  (set `self.CardRotation` _returnvalue_rotation)
  (bind (_direction _location _rotation) (`Timeline|ResetCard` :!via `PlayFromStart`)
    (:`Update`
      (`SceneComponent.K2_SetRelativeLocation` (`self.stone_slab`) (+ _location (`self.CardLocation`)) false false)
      (`SceneComponent.K2_SetRelativeRotation` (`self.stone_slab`) (`KismetMathLibrary.MakeRotator` 0.0 _rotation) false false)
      (set `self.IsTurned` false))))

(fn `ToggleCard`
  (bind (_returnvalue_roll _returnvalue_pitch) (`KismetMathLibrary.BreakRotator` (`SceneComponent.K2_GetComponentRotation` (`self.stone_slab`))))
  (set `self.IsClickable` (not (`self.IsClickable`)))
  (if (== _returnvalue_pitch 0.0)
    (`self.Turn Card`)
    (else
      (`self.Reset Card`))))

(fn `UserConstructionScript`
  (switch `/Game/Memory/E_CardTypes` (`self.CardType`)
    (:`NewEnumerator0`
      (`PrimitiveComponent.SetMaterial` (`self.Cube`) 0 "/Game/Memory/Images/bison_Mat.bison_Mat"))
    (:`NewEnumerator1`
      (`PrimitiveComponent.SetMaterial` (`self.Cube`) 0 "/Game/Memory/Images/cerf_Mat.cerf_Mat"))
    (:`NewEnumerator2`
      (`PrimitiveComponent.SetMaterial` (`self.Cube`) 0 "/Game/Memory/Images/sanglier_Mat.sanglier_Mat"))
    (:`NewEnumerator3`
      (`PrimitiveComponent.SetMaterial` (`self.Cube`) 0 "/Game/Memory/Images/gnou_Mat.gnou_Mat"))))