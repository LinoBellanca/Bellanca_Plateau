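; BP_MemoryGM is the manager for a memory card-matching game, enabling the mouse cursor and click events at BeginPlay.
; OnCardClicked stores the first card as PrevCard, then compares its CardType with that of the next clicked card.
; A match increments Score and destroys both cards, while a mismatch toggles both; either outcome clears PrevCard and prints a debug string.
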(event `self.ReceiveBeginPlay`
  (bind _returnvalue (`GameplayStatics.GetPlayerController` 0))
  (set `PlayerController.bEnableClickEvents` true _returnvalue)
  (set `PlayerController.bShowMouseCursor` true _returnvalue))

(fn `OnCardClicked`
  (params (Card :type "/Game/Memory/Carte/BP_Carte Object Reference"))
  (if (`KismetSystemLibrary.IsValid` (`self.PrevCard`))
    (if (`|EnumEquality` (`/Game/Memory/Carte/BP_Carte.CardType` Card) (`/Game/Memory/Carte/BP_Carte.CardType` (`self.PrevCard`)))
      (`KismetSystemLibrary.PrintString` "True")
      (bind _result (`/Engine/EditorBlueprintResources/StandardMacros.IncrementInt` (`self.Score`))
        (:`  `
          (set `self.Score` _result)
          (`self.K2_DestroyActor` Card)
          (`self.K2_DestroyActor` (`self.PrevCard`))
          (set `self.PrevCard` null)))
      (else
        (`KismetSystemLibrary.PrintString` "Fakse")
        (`/Game/Memory/Carte/BP_Carte.ToggleCard` Card)
        (`/Game/Memory/Carte/BP_Carte.ToggleCard` (`self.PrevCard`))
        (set `self.PrevCard` null)))
    (else
      (set `self.PrevCard` Card))))

(fn `UserConstructionScript`)