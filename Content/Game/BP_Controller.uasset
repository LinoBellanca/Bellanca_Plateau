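; BP_Controller is a controller Blueprint holding unfinished or disabled logic for orbiting the player's camera while the right mouse button is held.
; Its BeginPlay, Tick, LookYaw and LookPitch events are empty, so none of the logic runs.
; The disconnected nodes cast the player pawn to BP_Player and add scaled look-axis input as yaw or pitch world rotation on its SpringArm.
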(event `self.ReceiveBeginPlay`)

(event `EnhancedInput|/Game/Game/Inputs/LookYaw`
  (params (ActionValue :type "Float (double-precision)") (ElapsedSeconds :type "Float (double-precision)") (TriggeredSeconds :type "Float (double-precision)") (InputAction :type "InputAction Object Reference" :default "/Game/Game/Inputs/LookYaw.LookYaw")))

(event `EnhancedInput|/Game/Game/Inputs/LookPitch`
  (params (ActionValue :type "Float (double-precision)") (ElapsedSeconds :type "Float (double-precision)") (TriggeredSeconds :type "Float (double-precision)") (InputAction :type "InputAction Object Reference" :default "/Game/Game/Inputs/LookPitch.LookPitch")))

(fn `UserConstructionScript`)