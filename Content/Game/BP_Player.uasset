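; BP_Player is the player's camera pawn, with spring-arm zoom and orbit controls plus a T key that calls CyclePlayers on BP_GameMode.
; The mouse wheel steps a clamped CameraPosition, which Tick turns into a smoothly interpolated arm length.
; Holding right mouse lets mouse axes pitch the arm locally and yaw it in world space.
; Move axis events are empty, and the camera-relative AddMovementInput calls are disconnected.
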(event EventBeginPlay
  (bind _asbp_game_mode (Utilities|Casting|CastToBP_GameMode (Game|GetGameMode)))
  (Variables|Default|SetAs%20BP%20Game%20Mode _asbp_game_mode)
  (bind _asbp_controller (Utilities|Casting|CastToBP_Controller (Game|GetPlayerController 0)))
  (Variables|Default|SetAs%20BP%20Controller _asbp_controller))

(event EventTick
  (params (DeltaSeconds :type Float%20%28single-precision%29))
  (bind _springarm (Variables|Default|GetSpringArm))
  (Variables|/Script/Engine.SpringArmComponent|SetTargetArmLength _springarm (Math|Interpolation|FInterpTo (Variables|/Script/Engine.SpringArmComponent|GetTargetArmLength _springarm) (+ 1.2e+03 (* (* 3e+02 (Variables|Default|GetCameraPosition)) -1.0)) DeltaSeconds 2.0)))

(event Input|AxisEvents|InputAxisLookUp/DownMouse
  (params (AxisValue :type Float%20%28single-precision%29))
  (if (Game|Player|IsInputKeyDown (Variables|Default|GetAs%20BP%20Controller) "RightMouseButton")
    (Transformation|AddLocalRotation (Variables|Default|GetSpringArm) (Math|Rotator|MakeRotator 0.0 (* AxisValue 3.0) 0.0) false false)))

(event Input|AxisEvents|InputAxisTurnRight/LeftMouse
  (params (AxisValue :type Float%20%28single-precision%29))
  (if (Game|Player|IsInputKeyDown (Variables|Default|GetAs%20BP%20Controller) "RightMouseButton")
    (Transformation|AddWorldRotation (Variables|Default|GetSpringArm) (Math|Rotator|MakeRotator 0.0 0.0 (* AxisValue 3.0)) false false)))

(event Input|AxisEvents|InputAxisMoveForward/Backward
  (params (AxisValue :type Float%20%28single-precision%29)))

(event Input|AxisEvents|InputAxisMoveRight/Left
  (params (AxisValue :type Float%20%28single-precision%29)))

(event Input|MouseEvents|MouseWheelAxis
  (params (AxisValue :type Float%20%28single-precision%29))
  (bind _maxcamerapos (Variables|Default|GetMaxCameraPos))
  (bind _maxcamerapos_2 (Variables|Default|GetMaxCameraPos))
  (if (> AxisValue 0.0)
    (bind _result (Math|Integer|IncrementInt (Variables|Default|GetCameraPosition))
      (:%20%20
        (Variables|Default|SetCameraPosition (Math|Integer|Clamp(Integer) _result (* _maxcamerapos_2 -1) _maxcamerapos_2))))
    (elif (< AxisValue 0.0)
      (bind _result_2 (Math|Integer|DecrementInt (Variables|Default|GetCameraPosition))
        (:%20%20
          (Variables|Default|SetCameraPosition (Math|Integer|Clamp(Integer) _result_2 (* _maxcamerapos -1) _maxcamerapos)))))))

(event Input|KeyboardEvents|DebugKeyT
  (params (Key :type Key%20Structure :default "None") (ActionValue :type Input%20Action%20Value%20Structure)))

(event Input|KeyboardEvents|T
  (params (Key :type Key%20Structure :default "None"))
  (:Pressed
    (Default|CyclePlayers (Variables|Default|GetAs%20BP%20Game%20Mode))))

(fn ConstructionScript)