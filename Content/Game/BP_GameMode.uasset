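; Game mode for a turn-based dice board game, spawning one pawn per player, the die, and dice and score widgets.
; RollADiceAndMove adds the die result to the player's cell stored in the GameInstance, clamped to the board's last cell.
; MovePion saves the destination and starts single-cell steps forward or backward.
; On arrival it shows the end screen at the last cell, otherwise triggers the cell's action and cycles players if unmoved.
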(event `self.ReceiveBeginPlay`
  (bind _returnvalue (`KismetMathLibrary.RandomFloatInRange` 0.0 360.0))
  (bind _asbp_game_instance (cast `/Game/Game/BP_GameInstance` (`GameplayStatics.GetGameInstance`)))
  (bind _output_get (set `self.As BP Game Instance` _asbp_game_instance))
  (`/Game/Game/BP_GameInstance.GetPlayerCellNumberByPlayerID` _output_get 0)
  (`KismetSystemLibrary.Delay` 0.5)
  (for _index (range (`KismetArrayLibrary.Array_Length` (`/Game/Game/BP_GameInstance.PlayerList` (`self.As BP Game Instance`))))
    (bind _playercellnumber (`/Game/Game/BP_GameInstance.GetPlayerCellNumberByPlayerID` (`self.As BP Game Instance`) _index))
    (bind _celllocation (`/Game/CaseEtPlateau/BP_Board.GetCellPositionByNumber` (`self.Plateau`) _playercellnumber _index))
    (bind _returnvalue_2 (`|SpawnActorFromClass` "/Game/Characters/Cavenain/BP_Pion.BP_Pion_C" (`KismetMathLibrary.MakeTransform` (+ _celllocation (0.0 0.0 200.0))) "AlwaysSpawn" "MultiplyWithRoot" null null))
    ;[1 1 1] Créer la liste des pions en fonction du nombre de players
    (`KismetArrayLibrary.Array_Set` (`self.PionPlayer`) _index _returnvalue_2 true)
    (if (> (- (`KismetArrayLibrary.Array_Length` (`/Game/Game/BP_GameInstance.PlayerList` (`self.As BP Game Instance`))) 1) (`self.PlayerIDToPlay`))
      (`PrimitiveComponent.SetMaterial` (`Character.Mesh` (`|GetArrayItem` (`self.PionPlayer`) (`self.PlayerIDToPlay`))) 0 "/Game/Characters/Cavenain/Model/CM.CM")
      ;[1 1 1] S'il n'est pas le dernier, j'incrémente l'ID
      (bind _result (`/Engine/EditorBlueprintResources/StandardMacros.IncrementInt` (`self.PlayerIDToPlay`))
        (:`  `
          (set `self.PlayerIDToPlay` _result)))
      (else
        (`PrimitiveComponent.SetMaterial` (`Character.Mesh` (`|GetArrayItem` (`self.PionPlayer`) (`self.PlayerIDToPlay`))) 0 "/Game/Characters/Cavenain/Model/CM_2.CM_2")
        ;[1 1 1] S'il l'est, je  remet l'ID à 0
        (set `self.PlayerIDToPlay` 0))))
  (bind _returnvalue_3 (`|SpawnActorFromClass` "/Game/Dé/Bp_De.Bp_De_C" (`KismetMathLibrary.MakeTransform` (770.0 70.0 990.0) (`KismetMathLibrary.MakeRotator` _returnvalue _returnvalue _returnvalue)) "Undefined" "MultiplyWithRoot" null null))
  (set `self.Dice` _returnvalue_3)
  (bind _returnvalue_4 (`|CreateWidget` "/Game/Widgets/WB_Dice.WB_Dice_C"))
  (`UserWidget.AddToViewport` _returnvalue_4 0)
  (bind _returnvalue_5 (`|CreateWidget` "/Game/Widgets/WB_Score.WB_Score_C"))
  (`UserWidget.AddToViewport` _returnvalue_5 0))

(event `GetCellList`
  (params (IndexCase :type Integer))
  ;[0 0 0] Ancienne méthode de spawn
)

(event `ShowEndWidget`
  (bind _returnvalue (`|CreateWidget` "/Game/Widgets/WB_EndGame.WB_EndGame_C"))
  (`UserWidget.AddToViewport` _returnvalue 0)
  (set `PlayerController.bShowMouseCursor` true (`GameplayStatics.GetPlayerController` 0))
  (`self.DisableInput` (`GameplayStatics.GetPlayerPawn` 0) null))

(event `Move1by1`
  (params (`Cell Destination` :type Integer))
  (bind _playeridtoplay (`self.PlayerIDToPlay`))
  (bind _returnvalue (+ (`self.ActualCellNumber`) 1))
  (`/Game/Game/BP_GameInstance.SetPlayerCellNumberByPlayerID` (`self.As BP Game Instance`) _playeridtoplay _returnvalue)
  (bind _celllocation (`/Game/CaseEtPlateau/BP_Board.GetCellPositionByNumber` (`self.Plateau`) _returnvalue _playeridtoplay))
  ;[1 1 1] Déplacement du pion
  (`/Game/Characters/Cavenain/BP_Pion.MoveToTempCell` (`|GetArrayItem` (`self.PionPlayer`) (`self.PlayerIDToPlay`)) _celllocation 0))

(fn `CyclePlayers`
  (if (> (- (`KismetArrayLibrary.Array_Length` (`/Game/Game/BP_GameInstance.PlayerList` (`self.As BP Game Instance`))) 1) (`self.PlayerIDToPlay`))
    ;[1 1 1] S'il n'est pas le dernier, j'incrémente l'ID
    (bind _result (`/Engine/EditorBlueprintResources/StandardMacros.IncrementInt` (`self.PlayerIDToPlay`))
      (:`  `
        (set `self.PlayerIDToPlay` _result)))
    (else
      ;[1 1 1] S'il l'est, je  remet l'ID à 0
      (set `self.PlayerIDToPlay` 0))))

(fn `GoBack1By1`
  (params (FinalCell :type Integer))
  (bind _playeridtoplay (`self.PlayerIDToPlay`))
  (bind _celllocation (`/Game/CaseEtPlateau/BP_Board.GetCellPositionByNumber` (`self.Plateau`) (- (`self.ActualCellNumber`) 1) _playeridtoplay))
  (`/Game/Characters/Cavenain/BP_Pion.MoveToTempCell` (`|GetArrayItem` (`self.PionPlayer`) _playeridtoplay) _celllocation FinalCell)
  (set `self.ActualCellNumber` (- (`self.ActualCellNumber`) 1)))

(fn `GoOn1By1`
  (params (FinalCell :type Integer))
  (bind _playeridtoplay (`self.PlayerIDToPlay`))
  (bind _celllocation (`/Game/CaseEtPlateau/BP_Board.GetCellPositionByNumber` (`self.Plateau`) (+ (`self.ActualCellNumber`) 1) _playeridtoplay))
  (`/Game/Characters/Cavenain/BP_Pion.MoveToTempCell` (`|GetArrayItem` (`self.PionPlayer`) _playeridtoplay) _celllocation FinalCell)
  (set `self.ActualCellNumber` (+ (`self.ActualCellNumber`) 1)))

(fn `MovePion`
  (params (CellDestination :type Integer) (PlayerID :type Integer))
  ;[1 1 1] Sauvegarde du nouveau numéro de case/position sur le board
  (`/Game/Game/BP_GameInstance.SetPlayerCellNumberByPlayerID` (`self.As BP Game Instance`) PlayerID CellDestination)
  ;[1 1 1] Déterminer la position finale dans le board
  (bind _celllocation (`/Game/CaseEtPlateau/BP_Board.GetCellPositionByNumber` (`self.Plateau`) CellDestination PlayerID))
  (if (== (`self.ActualCellNumber`) CellDestination)
    ;[1 1 1] Déplacement du pion
    (`/Game/Characters/Cavenain/BP_Pion.MoveToNewCell` (`|GetArrayItem` (`self.PionPlayer`) PlayerID) _celllocation)
    (if (>= CellDestination (- (`KismetArrayLibrary.Array_Length` (`/Game/CaseEtPlateau/BP_Board.CellList` (`self.Plateau`))) 1))
      (`self.ShowEndWidget`)
      (else
        (`/Game/CaseEtPlateau/BP_Cell.Action` (`|GetArrayItem` (`/Game/CaseEtPlateau/BP_Board.CellList` (`self.Plateau`)) CellDestination) PlayerID)
        (if (== (`self.ActualCellNumber`) CellDestination)
          (`KismetSystemLibrary.PrintString` "Cycle")
          (`self.CyclePlayers`)
          (else
            (`KismetSystemLibrary.PrintString` "zzzz")))))
    (elif (< (`self.ActualCellNumber`) CellDestination)
      (`self.GoOn1By1` CellDestination)
      (else
        (`self.GoBack1By1` CellDestination)))))

(fn `RollADiceAndMove`
  (params (IDToPlay :type Integer))
  (locals (TempCellDestination :type Integer))
  (bind _playercellnumber (`/Game/Game/BP_GameInstance.GetPlayerCellNumberByPlayerID` (`self.As BP Game Instance`) IDToPlay))
  (set `self.ActualCellNumber` _playercellnumber)
  (bind _casesnombre (`/Game/CaseEtPlateau/BP_Board.GetCellNumber` (`self.Plateau`)))
  (bind _returnvalue (+ _playercellnumber (`/Game/Dé/Bp_De.ActualDiceResult` (`self.Dice`))))
  (bind _returnvalue_2 (- _casesnombre 1))
  (if (> _returnvalue _returnvalue_2)
    (set `local.TempCellDestination` _returnvalue_2)
    (else
      (set `local.TempCellDestination` _returnvalue)))
  (`self.MovePion` (`local.TempCellDestination`) (`self.PlayerIDToPlay`)))

(fn `UserConstructionScript`)